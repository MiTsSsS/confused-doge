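; Enemy character Blueprint with health, floating damage numbers and a death sequence.
; On BeginPlay it caches the damage container widget from its FloatingDamage widget component.
; While Hp remains, AnyDamage adds an animated damage widget to that container and subtracts Hp, then at zero plays a backwards death animation and destroys the actor after a delay.
; Attack is a stub that only prints a debug string.
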(event `Attack`
  (`KismetSystemLibrary.PrintString` "Attack"))

(event `self.ReceiveBeginPlay`
  (bind _aswbp_floating_damage_container (cast `/Game/UI/Combat/WBP_FloatingDamageContainer` (`WidgetComponent.GetWidget` (`self.FloatingDamage`))))
  (set `self.floatDamage` _aswbp_floating_damage_container))

(event `self.ReceiveAnyDamage`
  (params (Damage :type "Float (single-precision)") (DamageType :type "DamageType Object Reference") (InstigatedBy :type "Controller Object Reference") (DamageCauser :type "Actor Object Reference"))
  (if (> (`self.hp`) 0.0)
    (bind _returnvalue (`|CreateWidget` "/Game/UI/Combat/WBP_FloatingDamage.WBP_FloatingDamage_C" null Damage))
    (`PanelWidget.AddChild` (`/Game/UI/Combat/WBP_FloatingDamageContainer.StackBox_0` (`self.floatDamage`)) _returnvalue)
    (`/Game/UI/Combat/WBP_FloatingDamage.PlayAnim` _returnvalue)
    (bind _output_get (set `self.hp` (- (`self.hp`) Damage)))
    (if (<= _output_get 0.0)
      (`SkeletalMeshComponent.PlayAnimation` (`self.Mesh`) "/Game/Characters/Models/Enemy/Dying_Backwards.Dying_Backwards" false)
      (`KismetSystemLibrary.Delay` 3.0)
      (`self.K2_DestroyActor`)
      (else
        (`KismetSystemLibrary.PrintString` (`KismetStringLibrary.Concat_StrStr` "NEW HP: " (`KismetStringLibrary.Conv_DoubleToString` (`self.hp`))))))))

(fn `UserConstructionScript`)